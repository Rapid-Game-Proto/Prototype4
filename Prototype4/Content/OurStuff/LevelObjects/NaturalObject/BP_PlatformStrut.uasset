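; BP_PlatformStrut is a destructible level object that holds back a linked platform.
; Its DestroyObject override sets CanMove on LinkedPlatform, then runs the parent's destruction logic.
; A separate WallDoorSwitch event prints a debug string, hides the actor in game and plays a wall-transform sound once at its location.
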(event Custom|WallDoorSwitch
  ;[1 1 1] Wall Door switch
  (Development|PrintString "WallSwitched")
  (Rendering|SetActorHiddenInGame true)
  (Utilities|FlowControl|DoOnce false
    (:Completed
      (Audio|PlaySoundatLocation "/Game/OurStuff/Assets/Sounds/SC_WallTransform.SC_WallTransform" (Transformation|GetActorLocation) "0, 0, 0" 1.0 1.0 0.0 0 0 0 0))))

(event EventBeginPlay
  (|CallParentFunction) ; This node is disabled and will not be called.\nDrag off pins to build functionality.
)

(event Collision|EventActorBeginOverlap
  (params (OtherActor :type Actor%20Object%20Reference)))

(event EventTick
  (params (DeltaSeconds :type Float%20%28single-precision%29))
  (|CallParentFunction DeltaSeconds) ; This node is disabled and will not be called.\nDrag off pins to build functionality.
)

(fn ConstructionScript
  (|CallParentFunction))

(fn DestroyObject
  (Variables|/Game/OurStuff/Blueprints/LevelMovement/BP_MovingPlatform.BP_MovingPlatform_C|SetCanMove? (Variables|Default|GetLinkedPlatform) true)
  (|CallParentFunction))