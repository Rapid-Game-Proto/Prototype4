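; Breakable level object with health and a moving sweet spot, replaced by BP_GeometricBreakableObject when destroyed.
; Character overlap with Area shows a camera-facing health bar and places the sweet spot; leaving hides both.
; Random line traces toward the actor, confirmed by a camera visibility trace, position HitMesh on the visible surface.
; ObjectHit applies damage, scaled by SweetSpotMultiplier on misses, and flags Tick to relocate the spot.
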(event OnComponentBeginOverlap(Area)
  (params (OverlappedComponent :type Primitive%20Component%20Object%20Reference) (OtherActor :type Actor%20Object%20Reference) (OtherComp :type Primitive%20Component%20Object%20Reference) (OtherBodyIndex :type Integer) (bFromSweep :type Boolean) (SweepResult :type Hit%20Result%20Structure%20%28by%20ref%29))
  (Utilities|Casting|CastToBP_Character OtherActor)
  (CallFunction|LoadNewSweetSpot)
  (Development|SetHiddeninGame (Variables|Default|GetHealthBar) false false))

(event OnComponentEndOverlap(Area)
  (params (OverlappedComponent :type Primitive%20Component%20Object%20Reference) (OtherActor :type Actor%20Object%20Reference) (OtherComp :type Primitive%20Component%20Object%20Reference) (OtherBodyIndex :type Integer))
  (Utilities|Casting|CastToBP_Character OtherActor)
  (CallFunction|UnloadSweetSpot)
  (Development|SetHiddeninGame (Variables|Default|GetHealthBar) true false))

(event EventBeginPlay
  (Development|SetHiddeninGame (Variables|Default|GetHealthBar) true false))

(event EventTick
  (params (DeltaSeconds :type Float%20%28single-precision%29))
  (Utilities|FlowControl|Sequence
    (:then_0
      (CallFunction|UpdateHealthBar))
    (:then_1
      (if (Variables|Default|GetIsHit?)
        (CallFunction|LoadNewSweetSpot)
        (Variables|Default|SetIsHit? false)))))

(fn ConstructionScript)

(fn LoadNewSweetSpot
  (bind _returnvalue (Transformation|GetActorLocation))
  (Utilities|FlowControl|ForLoopwithBreak 0 (Variables|Default|GetLast%20Index) :!label _label
    (:LoopBody
      (bind _outhit (Collision|LineTraceByChannel (+ _returnvalue (* (Math|Random|RandomUnitVector) (Variables|Default|GetSweetSpotVariableTBD))) _returnvalue "TraceTypeQuery1" false 0 "None" false))
      (if (and (< (.Distance (Collision|BreakHitResult _outhit)) 225.0) (and (.bBlockingHit (Collision|BreakHitResult _outhit)) (== (.HitActor (Collision|BreakHitResult _outhit)) self)))
        (bind _returnvalue_2 (Actor|GetActorOfClass "/Game/OurStuff/Blueprints/BP_Character.BP_Character_C"))
        (bind _outhit_2 (Collision|LineTraceByChannel (Transformation|GetWorldLocation (Variables|/Game/OurStuff/Blueprints/BP_Character.BP_Character_C|GetCamera _returnvalue_2)) (.Location (Collision|BreakHitResult _outhit)) "TraceTypeQuery1" true 0 "None" false "(R=1.000000,G=0.000000,B=0.000000,A=1.000000)" "(R=0.000000,G=1.000000,B=0.000000,A=1.000000)" 1.0))
        (if (and (.bBlockingHit (Collision|BreakHitResult _outhit_2)) (== (.HitActor (Collision|BreakHitResult _outhit_2)) self))
          (Transformation|SetWorldLocation (Variables|Default|GetHitMesh) (.ImpactPoint (Collision|BreakHitResult _outhit_2)) false false)
          (goto _label Break))))))

(fn ObjectHit
  (params (SweetSpotHit? :type Boolean))
  (bind _basedamage (Variables|Default|GetBaseDamage))
  (Variables|Default|SetIsHit? true)
  (if SweetSpotHit?
    (CallFunction|TakeDamage _basedamage)
    (else
      (CallFunction|TakeDamage (* _basedamage (Variables|Default|GetSweetSpotMultiplier))))))

(fn TakeDamage
  (params (Amount :type Float%20%28double-precision%29))
  (Variables|Default|SetCurrentHealth (- (Variables|Default|GetCurrentHealth) Amount))
  (if (<= (- (Variables|Default|GetCurrentHealth) Amount) 0.0)
    (CallFunction|DestroyObject)))

(fn DestroyObject
  (Game|SpawnActorfromClass "/Game/OurStuff/LevelObjects/BP_GeometricBreakableObject.BP_GeometricBreakableObject_C" (Transformation|GetActorTransform) "Undefined" "MultiplyWithRoot" 0 0)
  (Actor|DestroyActor))

(fn UpdateHealthBar
  (bind _returnvalue (Actor|GetActorOfClass "/Game/OurStuff/Blueprints/BP_Character.BP_Character_C"))
  (Transformation|SetWorldRotation (Variables|Default|GetHealthBar) (Math|Rotator|FindLookatRotation (Transformation|GetWorldLocation (Variables|Default|GetHealthBar)) (Transformation|GetWorldLocation (Variables|/Game/OurStuff/Blueprints/BP_Character.BP_Character_C|GetCamera _returnvalue))) false false)
  (bind _aswbp_health_bar (Utilities|Casting|CastToWBP_HealthBar (UserInterface|GetWidget (Variables|Default|GetHealthBar))))
  (Variables|/Game/OurStuff/LevelObjects/WBP_HealthBar.WBP_HealthBar_C|SetPercentage _aswbp_health_bar (/ (Variables|Default|GetCurrentHealth) 2e+01)))

(fn UnloadSweetSpot
  (Transformation|SetWorldLocation (Variables|Default|GetHitMesh) (Transformation|GetWorldLocation (Variables|Default|GetStaticMesh)) false false))