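; BP_Girl is a sleeping girl actor that wakes when the alerted Sandman comes close.
; Each tick it finds BP_Sandman, reads PlayerFound from its BP_AIcontroller and checks whether the Sandman is within range of the girl's mesh.
; When both conditions hold, a DoOnce prints a message, plays a yawn sound, then after a short delay calls PlayerSpotted on BP_Gamemode.
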(event Collision|EventActorBeginOverlap
  (params (OtherActor :type Actor%20Object%20Reference)))

(event EventTick
  (params (DeltaSeconds :type Float%20%28single-precision%29))
  (bind _returnvalue (Actor|GetActorOfClass "/Game/OurStuff/AI/Sandman/BP_Sandman.BP_Sandman_C"))
  (bind _asbp_aicontroller (Utilities|Casting|CastToBP_AIcontroller (AI|GetAIController _returnvalue)))
  (if (Variables|/Game/OurStuff/AI/Sandman/BP_AIcontroller.BP_AIcontroller_C|GetPlayerFound _asbp_aicontroller)
    (if (<= (Math|Vector|Distance(Vector) (Transformation|GetActorLocation _returnvalue) (Transformation|GetWorldLocation (Variables|Default|GetStaticMesh))) 2e+02)
      (Utilities|FlowControl|DoOnce false
        (:Completed
          (Development|PrintString "Girl Woken")
          (Audio|PlaySound2D "/Game/OurStuff/Assets/Sounds/SC_GirlYawn.SC_GirlYawn" 1.0 1.0 0.0 0 0)
          (Utilities|FlowControl|Delay 3.0)
          (bind _asbp_gamemode (Utilities|Casting|CastToBP_Gamemode (Game|GetGameMode)))
          (Default|PlayerSpotted _asbp_gamemode))))))

(fn ConstructionScript)