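; A platform actor that moves toward an end location while a BP_Character is inside its trigger box and travels back when the character leaves.
; A timeline lerps the main mesh's relative location from its starting point to EndLocation, playing or reversing at a rate derived from DurationSecs.
; The construction script applies a configurable mesh, scale and rotation to the platform and to a reference mesh placed at the end location.
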(event OnComponentBeginOverlap(Box)
  (params (OverlappedComponent :type Primitive%20Component%20Object%20Reference) (OtherActor :type Actor%20Object%20Reference) (OtherComp :type Primitive%20Component%20Object%20Reference) (OtherBodyIndex :type Integer) (bFromSweep :type Boolean) (SweepResult :type Hit%20Result%20Structure%20%28by%20ref%29))
  (Utilities|Casting|CastToBP_Character OtherActor)
  (Components|Timeline|SetPlayRate (Variables|Default|GetMovePlatform) (/ 1.0 (Variables|Default|GetDuration%28secs%29)))
  (bind _movetrack (Timeline|MovePlatform Play)
    (:Update
      (Transformation|SetRelativeLocation (Variables|Default|GetMainPlatform) (Math|Vector|Lerp(Vector) (Variables|Default|GetStart%20Location) (Variables|Default|GetEnd%20Location) _movetrack) false false))))

(event OnComponentEndOverlap(Box)
  (params (OverlappedComponent :type Primitive%20Component%20Object%20Reference) (OtherActor :type Actor%20Object%20Reference) (OtherComp :type Primitive%20Component%20Object%20Reference) (OtherBodyIndex :type Integer))
  (Utilities|Casting|CastToBP_Character OtherActor)
  (Components|Timeline|SetPlayRate (Variables|Default|GetMovePlatform) (/ 1.0 (Variables|Default|GetDuration%28secs%29)))
  (bind _movetrack (Timeline|MovePlatform Reverse)
    (:Update
      (Transformation|SetRelativeLocation (Variables|Default|GetMainPlatform) (Math|Vector|Lerp(Vector) (Variables|Default|GetStart%20Location) (Variables|Default|GetEnd%20Location) _movetrack) false false))))

(event EventBeginPlay
  (Variables|Default|SetStart%20Location (Variables|/Script/Engine.SceneComponent|GetRelativeLocation (Variables|Default|GetMainPlatform))))

(fn ConstructionScript
  (bind _mainplatform (Variables|Default|GetMainPlatform))
  (bind _endplatformreference (Variables|Default|GetEndPlatformReference))
  (bind _new_mesh (Variables|Default|GetNew%20Mesh))
  (Components|StaticMesh|SetStaticMesh _mainplatform _new_mesh)
  (Components|StaticMesh|SetStaticMesh _endplatformreference _new_mesh)
  (Transformation|SetRelativeScale3D _mainplatform (Variables|Default|GetNew%20Scale))
  (Transformation|SetRelativeRotation _mainplatform (Variables|Default|GetNew%20Rotation) false false)
  (Transformation|SetRelativeLocation _endplatformreference (Variables|Default|GetEnd%20Location) false false))