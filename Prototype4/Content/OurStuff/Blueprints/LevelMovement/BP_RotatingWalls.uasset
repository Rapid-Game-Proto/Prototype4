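; BP_RotatingWalls is a wall actor that spins until BP_Character or BP_Sandman enters its trigger Box.
; Tick activates or deactivates the RotatingMovement component from the IsRotating flag, which the Box overlap events toggle.
; On entry, ResetTimeline eases only the pitch back to the rotation stored at BeginPlay, lerping from the current value each update.
; When either actor leaves the Box, rotation resumes.
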(event OnComponentBeginOverlap(Box)
  (params (OverlappedComponent :type Primitive%20Component%20Object%20Reference) (OtherActor :type Actor%20Object%20Reference) (OtherComp :type Primitive%20Component%20Object%20Reference) (OtherBodyIndex :type Integer) (bFromSweep :type Boolean) (SweepResult :type Hit%20Result%20Structure%20%28by%20ref%29))
  (bind _returnvalue (Transformation|GetActorRotation))
  (bind (_roll _pitch _yaw) (Math|Rotator|BreakRotator _returnvalue))
  (Utilities|Casting|CastToBP_Character OtherActor
    (:then
      _)
    (:CastFailed
      (Utilities|Casting|CastToBP_Sandman OtherActor)))
  (Variables|Default|SetIsRotating%20 false)
  ;[1 1 1] Smooth rotation reset
  (bind _alpha (Timeline|ResetTimeline Play)
    (:Update
      (Transformation|SetActorRotation (Math|Rotator|MakeRotator _roll (Math|Float|Lerp _pitch (.Pitch (Math|Rotator|BreakRotator (Variables|Default|GetInitialRotation))) _alpha) _yaw)))))

(event OnComponentEndOverlap(Box)
  (params (OverlappedComponent :type Primitive%20Component%20Object%20Reference) (OtherActor :type Actor%20Object%20Reference) (OtherComp :type Primitive%20Component%20Object%20Reference) (OtherBodyIndex :type Integer))
  (Utilities|Casting|CastToBP_Character OtherActor
    (:then
      _)
    (:CastFailed
      (Utilities|Casting|CastToBP_Sandman OtherActor)))
  (Variables|Default|SetIsRotating%20 true))

(event EventBeginPlay
  (Variables|Default|SetInitialRotation (Transformation|GetActorRotation))
  (Variables|Default|SetIsRotating%20 true))

(event EventTick
  (params (DeltaSeconds :type Float%20%28single-precision%29))
  (if (Variables|Default|GetIsRotating%20)
    (Components|Activation|Activate (Variables|Default|GetRotatingMovement) false)
    (else
      (Components|Activation|Deactivate (Variables|Default|GetRotatingMovement)))))

(fn ConstructionScript)