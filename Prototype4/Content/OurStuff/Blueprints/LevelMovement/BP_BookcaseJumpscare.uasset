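; BP_BookcaseJumpscare is a scare prop that drops a book from a bookcase when BP_Character enters its trigger box.
; A DoOnce enables physics and pushes the book, then after delays plays the fall sound, reports a "BookDropped" AI noise and disables physics.
; RestockBookshelf teleports the book using its BeginPlay transform plus the root's world location, prints that transform and rearms the DoOnce.
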(event OnComponentBeginOverlap(Box)
  (params (OverlappedComponent :type Primitive%20Component%20Object%20Reference) (OtherActor :type Actor%20Object%20Reference) (OtherComp :type Primitive%20Component%20Object%20Reference) (OtherBodyIndex :type Integer) (bFromSweep :type Boolean) (SweepResult :type Hit%20Result%20Structure%20%28by%20ref%29))
  (bind _book (Variables|Default|GetBook))
  (Utilities|Casting|CastToBP_Character OtherActor)
  (Utilities|FlowControl|DoOnce false
    (:Completed
      (Physics|SetSimulatePhysics _book true)
      (Physics|AddForce _book "0.000000,100.000000,0.000000" "None" false)
      (Utilities|FlowControl|Delay 0.9)
      (Audio|PlaySoundatLocation "/Game/OurStuff/Assets/Sounds/SC_BookFalls.SC_BookFalls" (Transformation|GetActorLocation) "0, 0, 0" 1.0 1.0 0.0 0 0 0 0)
      (Class|AISenseHearing|ReportNoiseEvent (Transformation|GetWorldLocation (Variables|Default|GetBook)) 1.0 self 0.0 "BookDropped")
      (Utilities|FlowControl|Delay 5.0)
      (Physics|SetSimulatePhysics _book false))))

(event Custom|ResetDropEvent
  (bind _book (Variables|Default|GetBook))
  (Utilities|FlowControl|DoOnce false) ; enters at Reset
)

(event EventBeginPlay
  (Variables|Default|SetBookOrigin (Transformation|GetRelativeTransform (Variables|Default|GetBook))))

(fn ConstructionScript)

(fn RestockBookshelf
  (bind _bookorigin (Variables|Default|GetBookOrigin))
  (bind _defaultsceneroot (Variables|Default|GetDefaultSceneRoot))
  (bind _returnvalue (Transformation|GetWorldTransform _defaultsceneroot))
  (bind _returnvalue_2 (+ (.location _returnvalue) (.location _bookorigin)))
  (Transformation|SetRelativeTransform (Variables|Default|GetBook) (Math|Transform|MakeTransform _returnvalue_2 (.rotation _bookorigin) (.scale _bookorigin)) false true)
  (Development|PrintString (Utilities|String|ToString(Transform) (Math|Transform|MakeTransform _returnvalue_2 (.rotation _bookorigin) (.scale _bookorigin))))
  (CallFunction|ResetDropEvent))