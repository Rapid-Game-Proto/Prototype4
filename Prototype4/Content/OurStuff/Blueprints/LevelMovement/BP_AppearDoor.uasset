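; BP_AppearDoor is an interactable door that toggles its state through a timeline when the player interacts nearby.
; The OpenDoorBox overlap with BP_Character enables input and opens a gate, and leaving disables input and closes it.
; Interact passes through that gate into a FlipFlop that alternately plays and reverses DoorTimeline, whose update output is unwired.
; The Wall component has query and physics collision enabled at BeginPlay.
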(event OnComponentBeginOverlap(OpenDoorBox)
  (params (OverlappedComponent :type Primitive%20Component%20Object%20Reference) (OtherActor :type Actor%20Object%20Reference) (OtherComp :type Primitive%20Component%20Object%20Reference) (OtherBodyIndex :type Integer) (bFromSweep :type Boolean) (SweepResult :type Hit%20Result%20Structure%20%28by%20ref%29))
  (Utilities|Casting|CastToBP_Character OtherActor)
  (Input|EnableInput (Game|GetPlayerController 0))
  (Utilities|FlowControl|Gate true) ; enters at Open
)

(event OnComponentEndOverlap(OpenDoorBox)
  (params (OverlappedComponent :type Primitive%20Component%20Object%20Reference) (OtherActor :type Actor%20Object%20Reference) (OtherComp :type Primitive%20Component%20Object%20Reference) (OtherBodyIndex :type Integer))
  (Utilities|Casting|CastToBP_Character OtherActor)
  (Input|DisableInput (Game|GetPlayerController 0))
  (Utilities|FlowControl|Gate true) ; enters at Close
)

(event Custom|Interact
  (Utilities|FlowControl|Gate true
    (:Exit
      (Utilities|FlowControl|FlipFlop
        (:A
          (Timeline|Door%20Timeline Play))
        (:B
          (Timeline|Door%20Timeline Reverse))))))

(event EventBeginPlay
  (Collision|SetCollisionEnabled (Variables|Default|GetWall) "QueryAndPhysics"))

(fn ConstructionScript)