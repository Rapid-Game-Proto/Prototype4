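; BP_Trap is a trap actor that holds a BP_Sandman in place or otherwise traps it for a set time on overlap.
; Box overlap calls TrapForTime on the Sandman, plays the skeletal mesh animation and destroys the trap once TrapTime passes.
; The physics Sphere has its starting rotation reapplied every Tick and its velocity zeroed shortly after a hit.
; A timer started on BeginPlay removes the trap if it is never triggered.
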(event OnComponentHit(Sphere)
  (params (HitComponent :type Primitive%20Component%20Object%20Reference) (OtherActor :type Actor%20Object%20Reference) (OtherComp :type Primitive%20Component%20Object%20Reference) (NormalImpulse :type Vector :default "0, 0, 0") (Hit :type Hit%20Result%20Structure%20%28by%20ref%29))
  (Utilities|FlowControl|Delay 0.2)
  (Physics|SetPhysicsLinearVelocity (Variables|Default|GetSphere) "0, 0, 0" false "None"))

(event OnComponentBeginOverlap(Box)
  (params (OverlappedComponent :type Primitive%20Component%20Object%20Reference) (OtherActor :type Actor%20Object%20Reference) (OtherComp :type Primitive%20Component%20Object%20Reference) (OtherBodyIndex :type Integer) (bFromSweep :type Boolean) (SweepResult :type Hit%20Result%20Structure%20%28by%20ref%29))
  (bind _traptime (Variables|Default|GetTrapTime))
  (bind _asbp_sandman (Utilities|Casting|CastToBP_Sandman OtherActor))
  (Default|TrapforTime _asbp_sandman _traptime)
  (Variables|Default|SetTrapActive true)
  (Audio|Components|Audio|Play (Variables|Default|GetSkeletalMesh) false)
  (Utilities|FlowControl|Delay _traptime)
  (Actor|DestroyActor))

(event EventBeginPlay
  (Variables|Default|SetStartRotation (Transformation|GetWorldRotation (Variables|Default|GetSphere)))
  (Utilities|Time|SetTimerbyFunctionName 0 "EndOfLife" 12.0))

(event Collision|EventActorBeginOverlap
  (params (OtherActor :type Actor%20Object%20Reference)))

(event EventTick
  (params (DeltaSeconds :type Float%20%28single-precision%29))
  (Transformation|SetWorldRotation (Variables|Default|GetSphere) (Variables|Default|GetStartRotation) false false))

(fn ConstructionScript)

(fn EndOfLife
  (if (not (Variables|Default|GetTrapActive))
    (Actor|DestroyActor)))