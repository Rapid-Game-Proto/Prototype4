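; BP_RotatingWalls is a wall actor that stops rotating while a BP_Character is inside its Box trigger.
; It records its rotation at BeginPlay.
; When the character enters the Box, it deactivates the RotatingMovement component and snaps the actor back to that initial rotation.
; When the character leaves, it reactivates RotatingMovement.
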(event OnComponentBeginOverlap(Box)
  (params (OverlappedComponent :type Primitive%20Component%20Object%20Reference) (OtherActor :type Actor%20Object%20Reference) (OtherComp :type Primitive%20Component%20Object%20Reference) (OtherBodyIndex :type Integer) (bFromSweep :type Boolean) (SweepResult :type Hit%20Result%20Structure%20%28by%20ref%29))
  (Utilities|Casting|CastToBP_Character OtherActor)
  (Components|Activation|Deactivate (Variables|Default|GetRotatingMovement))
  (Transformation|SetActorRotation (Variables|Default|GetInitialRotation)))

(event OnComponentEndOverlap(Box)
  (params (OverlappedComponent :type Primitive%20Component%20Object%20Reference) (OtherActor :type Actor%20Object%20Reference) (OtherComp :type Primitive%20Component%20Object%20Reference) (OtherBodyIndex :type Integer))
  (Utilities|Casting|CastToBP_Character OtherActor)
  (Components|Activation|Activate (Variables|Default|GetRotatingMovement) false))

(event EventBeginPlay
  (Variables|Default|SetInitialRotation (Transformation|GetActorRotation)))

(event EventTick
  (params (DeltaSeconds :type Float%20%28single-precision%29)))

(fn ConstructionScript)