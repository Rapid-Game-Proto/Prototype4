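; BP_Sandman is the Sandman AI character, which grows faster the longer it is active.
; On BeginPlay it attaches an idle sound to its capsule.
; Tick accumulates uptime and linearly ramps max walk speed from MinSpeed to MaxSpeed over roughly two minutes, then stops updating.
; TrapForTime accepts a duration but has no implementation here.
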(event EventBeginPlay
  (Audio|SpawnSoundAttached "/Game/OurStuff/Assets/Sounds/SC_SandmanIdle.SC_SandmanIdle" (Variables|Collision|GetCapsuleComponent) "None" "0, 0, 0" "0, 0, 0" "KeepRelativeOffset" false 1.0 1.0 0.0 0 0))

(event EventTick
  (params (DeltaSeconds :type Float%20%28single-precision%29))
  (if (not (> (Variables|Default|GetUptime) 1.2e+02))
    (bind _output_get (Variables|Default|SetUptime (+ DeltaSeconds (Variables|Default|GetUptime))))
    (Variables|/Script/Engine.CharacterMovementComponent|SetMaxWalkSpeed (Variables|Character|GetCharacterMovement) (Math|Float|Lerp (Variables|Default|GetMinSpeed) (Variables|Default|GetMaxSpeed) (/ _output_get 1.2e+02)))))

(fn ConstructionScript)

(fn TrapforTime
  (params (TimeTrapped :type Float%20%28double-precision%29)))