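; AI controller for the Weeping Angel enemy that tracks whether the player's view is facing it.
; On BeginPlay it runs the BT_WeepingAngel behavior tree and stores the BP_Character as the TargetActor blackboard key.
; Each tick it compares the camera's forward vector with the direction to the angel using a dot product, writing TargetHasVision without any occlusion trace.
; It also prints the dot value for debugging.
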(event EventBeginPlay
  (AI|RunBehaviorTree "/Game/OurStuff/AI/WeepingAngel/BT_WeepingAngel.BT_WeepingAngel")
  (bind _returnvalue (Actor|GetActorOfClass "/Game/OurStuff/Blueprints/BP_Character.BP_Character_C"))
  (bind _output_get (Variables|Default|SetCharacterRef _returnvalue))
  (AI|Components|Blackboard|SetValueasObject (Variables|Default|GetBlackboard) (Utilities|Name|MakeLiteralName "TargetActor") _output_get))

(event EventTick
  (params (DeltaSeconds :type Float%20%28single-precision%29))
  (CallFunction|HandlePlayerVisionSense))

(fn ConstructionScript)

(fn HandlePlayerVisionSense
  (bind _characterref (Variables|Default|GetCharacterRef))
  (bind _airef (Variables|Default|GetAIRef))
  (bind _returnvalue (Transformation|GetActorLocation _airef))
  (bind _returnvalue_2 (Transformation|GetActorLocation _characterref))
  (bind _camera (Variables|/Game/OurStuff/Blueprints/BP_Character.BP_Character_C|GetCamera _characterref))
  (bind _returnvalue_3 (Math|Vector|GetForwardVector _camera))
  (bind _returnvalue_4 (- _returnvalue _returnvalue_2))
  (bind _returnvalue_5 (Math|Vector|Normalize _returnvalue_4))
  (bind _returnvalue_6 (Math|Vector|DotProduct _returnvalue_5 _returnvalue_3))
  (bind _returnvalue_7 (Math|Float|InRange(Float) _returnvalue_6 0.2 1.0))
  (AI|Components|Blackboard|SetValueasBool (Variables|Default|GetBlackboard) (Utilities|Name|MakeLiteralName "TargetHasVision") _returnvalue_7)
  (Development|PrintString (Utilities|String|ToString(Float) _returnvalue_6))
  (if _returnvalue_7
    _))