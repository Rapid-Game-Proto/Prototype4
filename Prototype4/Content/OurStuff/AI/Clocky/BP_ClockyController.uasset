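; AI controller for the Clocky enemy that runs its behavior tree and feeds it player state through the blackboard.
; BeginPlay stores the player character as the target and enables movement.
; Each tick updates whether the player's camera faces Clocky, using a dot product, and whether the player is inside its active area.
; ResetAttack uses a DoOnce and delay to re-enable movement and reset both the ring task and Clocky's ring.
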(event Custom|ResetAttack
  (params (RingTaskRef :type BT%20Task%20Ring%20Object%20Reference))
  (Utilities|FlowControl|DoOnce false :!label _label
    (:Completed
      (Utilities|FlowControl|Delay 5.0)
      (CallFunction|ResetClockAttackCycle RingTaskRef)
      (Default|ResetRing (Variables|Default|GetAIRef))
      (goto _label Reset))))

(event EventBeginPlay
  (bind _blackboard (Variables|Default|GetBlackboard))
  (AI|RunBehaviorTree "/Game/OurStuff/AI/Clocky/BT_Clocky.BT_Clocky")
  (bind _returnvalue (Actor|GetActorOfClass "/Game/OurStuff/Blueprints/BP_Character.BP_Character_C"))
  (bind _output_get (Variables|Default|SetCharacterRef _returnvalue))
  (AI|Components|Blackboard|SetValueasObject _blackboard (Utilities|Name|MakeLiteralName "TargetActor") _output_get)
  (AI|Components|Blackboard|SetValueasBool _blackboard (Utilities|Name|MakeLiteralName "CanMove") true))

(event EventTick
  (params (DeltaSeconds :type Float%20%28single-precision%29))
  (CallFunction|HandlePlayerVisionSense)
  (CallFunction|HandlePlayerinRangeSense))

(fn ConstructionScript)

(fn HandlePlayerVisionSense
  (bind _characterref (Variables|Default|GetCharacterRef))
  (AI|Components|Blackboard|SetValueasBool (Variables|Default|GetBlackboard) (Utilities|Name|MakeLiteralName "TargetHasVision") (Math|Float|InRange(Float) (Math|Vector|DotProduct (Math|Vector|Normalize (- (Transformation|GetActorLocation (Variables|Default|GetAIRef)) (Transformation|GetActorLocation _characterref))) (Math|Vector|GetForwardVector (Variables|/Game/OurStuff/Blueprints/BP_Character.BP_Character_C|GetCamera _characterref))) 0.4 1.0)))

(fn HandlePlayerinRangeSense
  (AI|Components|Blackboard|SetValueasBool (Variables|Default|GetBlackboard) (Utilities|Name|MakeLiteralName "TargetInRange") (Variables|/Game/OurStuff/AI/Clocky/BP_ClockyActiveArea.BP_ClockyActiveArea_C|GetIsPlayerInRange (Variables|/Game/OurStuff/AI/Clocky/BP_ClockyComponent.BP_ClockyComponent_C|GetActiveArea (Variables|/Game/OurStuff/AI/Clocky/BP_Clocky.BP_Clocky_C|GetBP_ClockyComponent (Variables|Default|GetAIRef))))))

(fn ResetClockAttackCycle
  (params (RingTask :type BT%20Task%20Ring%20Object%20Reference))
  (AI|Components|Blackboard|SetValueasBool (Variables|Default|GetBlackboard) (Utilities|Name|MakeLiteralName "CanMove") true)
  (Default|ResetRing RingTask))