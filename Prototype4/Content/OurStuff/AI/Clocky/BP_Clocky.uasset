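; BP_Clocky is an AI clock character that rings to emit a noise event at its location and can be broken when hit.
; Its detection overlap toggles CanAttack on the BP_ClockyController blackboard as the player enters or leaves.
; Ringing plays audio and reports one "TargetLocation" noise until ResetRing stops it and re-arms the attack.
; Tick checks player camera proximity, which gates ObjectHit setting IsBroken on itself and the blackboard.
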(event OnComponentBeginOverlap(PlayerDetection)
  (params (OverlappedComponent :type Primitive%20Component%20Object%20Reference) (OtherActor :type Actor%20Object%20Reference) (OtherComp :type Primitive%20Component%20Object%20Reference) (OtherBodyIndex :type Integer) (bFromSweep :type Boolean) (SweepResult :type Hit%20Result%20Structure%20%28by%20ref%29))
  ;[1 1 1] Player Detection
  (Utilities|Casting|CastToBP_Character OtherActor)
  (bind _asbp_clocky_controller (Utilities|Casting|CastToBP_ClockyController (Pawn|GetController)))
  (AI|Components|Blackboard|SetValueasBool (Variables|/Script/AIModule.AIController|GetBlackboard _asbp_clocky_controller) (Utilities|Name|MakeLiteralName "CanAttack") true)
  (Variables|Default|SetInAttackRange true))

(event OnComponentEndOverlap(PlayerDetection)
  (params (OverlappedComponent :type Primitive%20Component%20Object%20Reference) (OtherActor :type Actor%20Object%20Reference) (OtherComp :type Primitive%20Component%20Object%20Reference) (OtherBodyIndex :type Integer))
  ;[1 1 1] Player Detection
  (Utilities|Casting|CastToBP_Character OtherActor)
  (bind _asbp_clocky_controller (Utilities|Casting|CastToBP_ClockyController (Pawn|GetController)))
  (AI|Components|Blackboard|SetValueasBool (Variables|/Script/AIModule.AIController|GetBlackboard _asbp_clocky_controller) (Utilities|Name|MakeLiteralName "CanAttack") false)
  (Variables|Default|SetInAttackRange false))

(event Custom|PlayRingSound
  ;[1 1 1] Sound Management
  (Utilities|FlowControl|Sequence
    (:then_0
      (Utilities|FlowControl|DoOnce false
        (:Completed
          (Class|AISenseHearing|ReportNoiseEvent (Transformation|GetWorldLocation (Variables|Character|GetMesh)) 1.0 self 0.0 "TargetLocation"))))
    (:then_1
      (Audio|Components|Audio|Play (Variables|Default|GetClockRing) 0.0))))

(event Custom|ResetRing
  ;[1 1 1] Sound Management
  (Audio|Components|Audio|Stop (Variables|Default|GetClockRing))
  (if (Variables|Default|GetInAttackRange)
    (bind _asbp_clocky_controller (Utilities|Casting|CastToBP_ClockyController (Pawn|GetController)))
    (AI|Components|Blackboard|SetValueasBool (Variables|/Script/AIModule.AIController|GetBlackboard _asbp_clocky_controller) (Utilities|Name|MakeLiteralName "CanAttack") true)
    (Utilities|FlowControl|DoOnce false) ; enters at Reset
    (else
      (Utilities|FlowControl|DoOnce false) ; enters at Reset
    )))

(event EventBeginPlay
  ;[1 1 1] Begin Play
  (bind _asbp_clocky_controller (Utilities|Casting|CastToBP_ClockyController (Pawn|GetController)))
  (Variables|/Game/OurStuff/AI/Clocky/BP_ClockyController.BP_ClockyController_C|SetAIRef _asbp_clocky_controller self)
  (bind _asbp_character (Utilities|Casting|CastToBP_Character (Game|GetPlayerCharacter 0)))
  (Variables|Default|SetPlayerRef _asbp_character)
  (Variables|Default|SetStartTransform (Transformation|GetActorTransform))
  (Audio|Components|Audio|Stop (Variables|Default|GetClockRing))
  (Variables|/Game/OurStuff/AI/Clocky/BP_ClockyComponent.BP_ClockyComponent_C|SetActiveArea (Variables|Default|GetBP_ClockyComponent) (Variables|Default|GetActiveAreaRef)))

(event EventTick
  (params (DeltaSeconds :type Float%20%28single-precision%29))
  (Utilities|FlowControl|Sequence
    (:then_0
      ;[1 1 1] Get Player Range
      (Variables|Default|SetPlayerInRange? (<= (Math|Vector|Distance(Vector) (Transformation|GetWorldLocation (Variables|Character|GetMesh)) (Transformation|GetWorldLocation (Variables|/Game/OurStuff/Blueprints/BP_Character.BP_Character_C|GetCamera (Variables|Default|GetPlayerRef)))) 2e+02)))))

(fn ConstructionScript)

(fn ObjectHit
  (if (Variables|Default|GetPlayerInRange?)
    (Development|PrintString "CLOCK GOT HITTEN")
    (Variables|Default|SetIsBroken? true)
    (bind _asbp_clocky_controller (Utilities|Casting|CastToBP_ClockyController (Pawn|GetController)))
    (AI|Components|Blackboard|SetValueasBool (Variables|/Script/AIModule.AIController|GetBlackboard _asbp_clocky_controller) (Utilities|Name|MakeLiteralName "IsBroken") true)))