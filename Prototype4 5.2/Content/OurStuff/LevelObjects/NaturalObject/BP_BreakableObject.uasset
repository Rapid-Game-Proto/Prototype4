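; Breakable world object the player damages, with bonus damage for hitting a sweet spot, swapped for BreakableBP when destroyed.
; While the player is inside Area, random line traces move HitMesh to a surface point visible to the camera, relocating it after each hit.
; Tick detects aim by trace or camera dot product, which ObjectHit uses to choose damage.
; Camera-facing widgets show health when aimed at and the sweet spot when in range.
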(event OnComponentBeginOverlap(Area)
  (params (OverlappedComponent :type Primitive%20Component%20Object%20Reference) (OtherActor :type Actor%20Object%20Reference) (OtherComp :type Primitive%20Component%20Object%20Reference) (OtherBodyIndex :type Integer) (bFromSweep :type Boolean) (SweepResult :type Hit%20Result%20Structure%20%28by%20ref%29))
  ;[1 1 1] Collision (Range)
  (bind _asbp_character (Utilities|Casting|CastToBP_Character OtherActor))
  (CallFunction|LoadNewSweetSpot)
  (Variables|Default|SetInRange? true)
  (Variables|/Game/OurStuff/Blueprints/BP_Character.BP_Character_C|SetIsClosetoBreakable _asbp_character true))

(event OnComponentEndOverlap(Area)
  (params (OverlappedComponent :type Primitive%20Component%20Object%20Reference) (OtherActor :type Actor%20Object%20Reference) (OtherComp :type Primitive%20Component%20Object%20Reference) (OtherBodyIndex :type Integer))
  ;[1 1 1] Collision (Range)
  (bind _asbp_character (Utilities|Casting|CastToBP_Character OtherActor))
  (CallFunction|UnloadSweetSpot)
  (Variables|Default|SetInRange? false)
  (Variables|/Game/OurStuff/Blueprints/BP_Character.BP_Character_C|SetIsClosetoBreakable _asbp_character false))

(event EventBeginPlay
  (Development|SetHiddeninGame (Variables|Default|GetHealthBar) true false)
  (CallFunction|UnloadSweetSpot)
  (Transformation|SetWorldScale3D (Variables|Default|GetHealthBar) "0.200000,0.200000,-0.020000")
  (Development|SetHiddeninGame (Variables|Default|GetHitMesh) true false)
  (Transformation|SetWorldScale3D (Variables|Default|GetHitMesh) "0.200000,0.200000,0.200000")
  (Transformation|SetWorldScale3D (Variables|Default|GetArea) (+ (Transformation|GetWorldScale (Variables|Default|GetStaticMesh)) 3.25))
  (bind _returnvalue (Actor|GetActorOfClass "/Game/OurStuff/Blueprints/BP_Character.BP_Character_C"))
  (Variables|Default|SetCharacterRef _returnvalue))

(event EventTick
  (params (DeltaSeconds :type Float%20%28single-precision%29))
  (bind _characterref (Variables|Default|GetCharacterRef))
  (bind _camera (Variables|/Game/OurStuff/Blueprints/BP_Character.BP_Character_C|GetCamera _characterref))
  (Utilities|FlowControl|Sequence
    (:then_0
      ;[1 1 1] General Tick Update Functions
      (CallFunction|UpdateHealthBar)
      (CallFunction|UpdateSweetSpot))
    (:then_1
      (if (Variables|Default|GetIsHit?)
        (CallFunction|LoadNewSweetSpot)
        (Variables|Default|SetIsHit? false)))
    (:then_2
      (if (Variables|Default|GetInRange?)
        (Utilities|FlowControl|Sequence
          (:then_0
            ;[1 1 1] Check Looking At By Trace
            (bind _outhit (Collision|LineTraceByChannel (Transformation|GetWorldLocation (Variables|/Script/Engine.Character|GetCapsuleComponent _characterref)) (* (Variables|/Game/OurStuff/Blueprints/BP_Character.BP_Character_C|GetLookDir _characterref) (* 1e+05 1e+05)) "TraceTypeQuery1" true 0 "None" false "(R=1.000000,G=0.000000,B=0.000000,A=1.000000)" "(R=0.000000,G=1.000000,B=0.000000,A=1.000000)" 1.0))
            (if (and (.bBlockingHit (Collision|BreakHitResult _outhit)) (== (.HitActor (Collision|BreakHitResult _outhit)) self))
              (Variables|Default|SetLookingAt? true)
              (if (== (.HitComponent (Collision|BreakHitResult _outhit)) (Variables|Default|GetHitMesh))
                (Variables|Default|SetLookingAtSweetSpotByTrace?? true)
                (else
                  (Variables|Default|SetLookingAtSweetSpotByTrace?? false :!label _label)))
              (else
                (Variables|Default|SetLookingAt? false)
                (goto _label))))
          (:then_1
            ;[1 1 1] Check Looking At By Dot Product
            (Variables|Default|SetLookingAtSweetSpotByDot? (Math|Float|InRange(Float) (Math|Vector|DotProduct (Math|Vector|Normalize (- (Transformation|GetWorldLocation (Variables|Default|GetSweetSpotWidget)) (Transformation|GetWorldLocation _camera))) (Math|Vector|GetForwardVector _camera)) 0.998 1.0))))))))

(fn ConstructionScript)

(fn LoadNewSweetSpot
  (bind _returnvalue (Transformation|GetActorLocation))
  (Utilities|FlowControl|ForLoopwithBreak 0 (Variables|Default|GetLast%20Index) :!label _label
    (:LoopBody
      (bind _outhit (Collision|LineTraceByChannel (+ _returnvalue (* (Math|Random|RandomUnitVector) (Variables|Default|GetSweetSpotVariableTBD))) _returnvalue "TraceTypeQuery1" true 0 "None" false))
      (if (and (< (.Distance (Collision|BreakHitResult _outhit)) 225.0) (and (.bBlockingHit (Collision|BreakHitResult _outhit)) (== (.HitActor (Collision|BreakHitResult _outhit)) self)))
        (bind _returnvalue_2 (Actor|GetActorOfClass "/Game/OurStuff/Blueprints/BP_Character.BP_Character_C"))
        (bind _outhit_2 (Collision|LineTraceByChannel (Transformation|GetWorldLocation (Variables|/Game/OurStuff/Blueprints/BP_Character.BP_Character_C|GetCamera _returnvalue_2)) (.Location (Collision|BreakHitResult _outhit)) "TraceTypeQuery1" false 0 "None" false "(R=1.000000,G=0.000000,B=0.000000,A=1.000000)" "(R=0.000000,G=1.000000,B=0.000000,A=1.000000)" 1.0))
        (if (and (.bBlockingHit (Collision|BreakHitResult _outhit_2)) (== (.HitActor (Collision|BreakHitResult _outhit_2)) self))
          (Transformation|SetWorldLocation (Variables|Default|GetHitMesh) (.ImpactPoint (Collision|BreakHitResult _outhit_2)) false false)
          (goto _label Break))))))

(fn ObjectHit
  (params (SweetSpotHit? :type Boolean))
  (bind _basedamage (Variables|Default|GetBaseDamage))
  (bind _characterref (Variables|Default|GetCharacterRef))
  (if (and (Variables|Default|GetInRange?) (Variables|Default|GetLookingAt?))
    (Variables|Default|SetIsHit? true)
    (if (or (Variables|Default|GetLookingAtSweetSpotByTrace??) (Variables|Default|GetLookingAtSweetSpotByDot?))
      (Variables|/Game/OurStuff/Blueprints/BP_Character.BP_Character_C|SetLastHitSuccess? _characterref true)
      (Development|PrintString "Hit Sweat Spot")
      (CallFunction|TakeDamage (* _basedamage (Variables|Default|GetSweetSpotMultiplier)))
      (else
        (Variables|/Game/OurStuff/Blueprints/BP_Character.BP_Character_C|SetLastHitSuccess? _characterref false)
        (Development|PrintString "Didnt Hit Sweat Spot")
        (CallFunction|TakeDamage _basedamage)))))

(fn TakeDamage
  (params (Amount :type Float%20%28double-precision%29))
  (Variables|Default|SetCurrentHealth (- (Variables|Default|GetCurrentHealth) Amount))
  (if (<= (- (Variables|Default|GetCurrentHealth) Amount) 0.0)
    (CallFunction|DestroyObject)))

(fn DestroyObject
  (Game|SpawnActorfromClass (Variables|Default|GetBreakableBP) (Transformation|GetWorldTransform (Variables|Default|GetStaticMesh)) "Undefined" "MultiplyWithRoot" 0 0)
  (Actor|DestroyActor))

(fn UpdateHealthBar
  (Utilities|FlowControl|Sequence
    (:then_0
      (bind _returnvalue (Actor|GetActorOfClass "/Game/OurStuff/Blueprints/BP_Character.BP_Character_C"))
      (Transformation|SetWorldRotation (Variables|Default|GetHealthBar) (Math|Rotator|FindLookatRotation (Transformation|GetWorldLocation (Variables|Default|GetHealthBar)) (Transformation|GetWorldLocation (Variables|/Game/OurStuff/Blueprints/BP_Character.BP_Character_C|GetCamera _returnvalue))) false false)
      (bind _aswbp_health_bar (Utilities|Casting|CastToWBP_HealthBar (UserInterface|GetWidget (Variables|Default|GetHealthBar))))
      (Variables|/Game/OurStuff/LevelObjects/Misc/WBP_HealthBar.WBP_HealthBar_C|SetPercentage _aswbp_health_bar (/ (Variables|Default|GetCurrentHealth) 2e+01)))
    (:then_1
      (Development|SetHiddeninGame (Variables|Default|GetHealthBar) (not (and (Variables|Default|GetInRange?) (Variables|Default|GetLookingAt?))) false))))

(fn UnloadSweetSpot
  (Transformation|SetWorldLocation (Variables|Default|GetHitMesh) (Transformation|GetWorldLocation (Variables|Default|GetStaticMesh)) false false))

(fn UpdateSweetSpot
  (bind _sweetspotwidget (Variables|Default|GetSweetSpotWidget))
  (Utilities|FlowControl|Sequence
    (:then_0
      (bind _returnvalue (Actor|GetActorOfClass "/Game/OurStuff/Blueprints/BP_Character.BP_Character_C"))
      (Transformation|SetWorldRotation _sweetspotwidget (Math|Rotator|FindLookatRotation (Transformation|GetWorldLocation _sweetspotwidget) (Transformation|GetWorldLocation (Variables|/Game/OurStuff/Blueprints/BP_Character.BP_Character_C|GetCamera _returnvalue))) false false))
    (:then_1
      (Development|SetHiddeninGame (Variables|Default|GetSweetSpotWidget) (not (Variables|Default|GetInRange?)) false))))