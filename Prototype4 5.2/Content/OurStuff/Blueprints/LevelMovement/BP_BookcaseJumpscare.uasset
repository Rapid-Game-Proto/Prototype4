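; BP_BookcaseJumpscare is a jumpscare prop that drops a book when the player character overlaps its trigger box.
; The overlap enables physics on the Book and applies a sideways force.
; After a short delay, a DoOnce plays the falling-book sound and reports an AI noise event tagged TargetLocation at the actor's location.
; Only the sound and noise are limited to once, not the physics push.
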(event OnComponentBeginOverlap(Box)
  (params (OverlappedComponent :type Primitive%20Component%20Object%20Reference) (OtherActor :type Actor%20Object%20Reference) (OtherComp :type Primitive%20Component%20Object%20Reference) (OtherBodyIndex :type Integer) (bFromSweep :type Boolean) (SweepResult :type Hit%20Result%20Structure%20%28by%20ref%29))
  (bind _book (Variables|Default|GetBook))
  (Utilities|Casting|CastToBP_Character OtherActor)
  (Physics|SetSimulatePhysics _book true)
  (Physics|AddForce _book "0.000000,100.000000,0.000000" "None" false)
  (Utilities|FlowControl|Delay 0.9)
  (Utilities|FlowControl|DoOnce false
    (:Completed
      (Audio|PlaySoundatLocation "/Game/OurStuff/Assets/Sounds/SC_BookFalls.SC_BookFalls" (Transformation|GetActorLocation) "0, 0, 0" 1.0 1.0 0.0 0 0 0 0)
      (Class|AISenseHearing|ReportNoiseEvent (Transformation|GetActorLocation) 1.0 self 0.0 "TargetLocation"))))

(fn ConstructionScript)