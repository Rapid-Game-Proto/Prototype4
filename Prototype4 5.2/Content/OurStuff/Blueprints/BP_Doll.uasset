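; BP_Doll is a one-time interactable doll that advances the player to the next level.
; Interact starts a self-recalling short-delay loop that yaws it toward the player, plays a giggle, then calls NextLevel on BP_Gamemode after a pause.
; Box overlaps toggle a widget that Tick turns toward the camera.
; Tick's outline overlay check requires both zero overlaps and the player overlapping, so it never applies.
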(event OnComponentBeginOverlap(Box)
  (params (OverlappedComponent :type Primitive%20Component%20Object%20Reference) (OtherActor :type Actor%20Object%20Reference) (OtherComp :type Primitive%20Component%20Object%20Reference) (OtherBodyIndex :type Integer) (bFromSweep :type Boolean) (SweepResult :type Hit%20Result%20Structure%20%28by%20ref%29))
  ;[1 1 1] Widget visability + rotation
  (Utilities|Casting|CastToBP_Character OtherActor)
  (Development|SetHiddeninGame (Variables|Default|GetWidget) false false))

(event OnComponentEndOverlap(Box)
  (params (OverlappedComponent :type Primitive%20Component%20Object%20Reference) (OtherActor :type Actor%20Object%20Reference) (OtherComp :type Primitive%20Component%20Object%20Reference) (OtherBodyIndex :type Integer))
  ;[1 1 1] Widget visability + rotation
  (Utilities|Casting|CastToBP_Character OtherActor)
  (Development|SetHiddeninGame (Variables|Default|GetWidget) true false))

(event Custom|Face%20Player
  ;[1 1 1] Face Player
  (Transformation|SetActorRotation (Math|Rotator|MakeRotator 0.0 0.0 (.yaw (Math|Interpolation|RInterpTo (Transformation|GetActorRotation) (Math|Rotator|FindLookatRotation (Transformation|GetActorLocation) (Transformation|GetActorLocation (Variables|Default|GetAs%20BP%20Character))) (Utilities|Time|GetWorldDeltaSeconds) 2e+01))))
  (Utilities|FlowControl|Delay 0.001)
  (CallFunction|FacePlayer))

(event Custom|Interact
  ;[1 1 1] Comment
  (Utilities|FlowControl|DoOnce false
    (:Completed
      (bind _asbp_character (Utilities|Casting|CastToBP_Character (Game|GetPlayerCharacter 0)))
      (Variables|Default|SetAs%20BP%20Character _asbp_character)
      (CallFunction|FacePlayer)
      (Audio|PlaySound2D "/Game/OurStuff/Assets/Sounds/SC_DollGiggle.SC_DollGiggle" 1.0 1.0 0.0 0 0)
      (Utilities|FlowControl|Delay 2.5)
      (bind _asbp_gamemode (Utilities|Casting|CastToBP_Gamemode (Game|GetGameMode)))
      (Default|NextLevel _asbp_gamemode))))

(event EventTick
  (params (DeltaSeconds :type Float%20%28single-precision%29))
  (bind _box (Variables|Default|GetBox))
  (bind _overlappingactors (Collision|GetOverlappingActors _box 0 :!class /Script/Engine.PrimitiveComponent))
  ;[1 1 1] Widget visability + rotation
  (Utilities|FlowControl|Sequence
    (:then_0
      (if (and (== (Utilities|Array|Length _overlappingactors) 0) (Utilities|Array|ContainsItem _overlappingactors (Variables|Default|GetAs%20BP%20Character)))
        (Rendering|Material|SetOverlayMaterial (Variables|Default|GetStaticMesh) "/Game/OurStuff/Assets/Materials/M_Outline_Inst.M_Outline_Inst" :!class /Script/Engine.MeshComponent)
        (else
          (Rendering|Material|SetOverlayMaterial (Variables|Default|GetStaticMesh) 0 :!class /Script/Engine.MeshComponent))))
    (:then_1
      (Transformation|SetWorldRotation (Variables|Default|GetWidget) (Math|Rotator|FindLookatRotation (Transformation|GetWorldLocation (Variables|Default|GetWidget)) (Transformation|GetWorldLocation (Variables|/Script/Engine.PlayerCameraManager|GetTransformComponent (Game|GetPlayerCameraManager 0)))) false false))))

(fn ConstructionScript)