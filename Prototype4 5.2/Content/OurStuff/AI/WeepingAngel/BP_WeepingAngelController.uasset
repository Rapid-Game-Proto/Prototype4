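; AI controller for the Weeping Angel enemy, running its behavior tree with the player character as TargetActor.
; Each tick it writes two blackboard flags for the tree to read.
; TargetHasVision comes from a dot product between the player camera's forward vector and the direction to the angel, approximating whether the player faces it.
; TargetInRange mirrors the player-in-range state of the angel component's origin area.
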(event EventBeginPlay
  (AI|RunBehaviorTree "/Game/OurStuff/AI/WeepingAngel/BT_WeepingAngel.BT_WeepingAngel")
  (bind _returnvalue (Actor|GetActorOfClass "/Game/OurStuff/Blueprints/BP_Character.BP_Character_C"))
  (bind _output_get (Variables|Default|SetCharacterRef _returnvalue))
  (AI|Components|Blackboard|SetValueasObject (Variables|Default|GetBlackboard) (Utilities|Name|MakeLiteralName "TargetActor") _output_get))

(event EventTick
  (params (DeltaSeconds :type Float%20%28single-precision%29))
  (CallFunction|HandlePlayerVisionSense)
  (CallFunction|HandlePlayerinRangeSense))

(fn ConstructionScript)

(fn HandlePlayerVisionSense
  (bind _characterref (Variables|Default|GetCharacterRef))
  (AI|Components|Blackboard|SetValueasBool (Variables|Default|GetBlackboard) (Utilities|Name|MakeLiteralName "TargetHasVision") (Math|Float|InRange(Float) (Math|Vector|DotProduct (Math|Vector|Normalize (- (Transformation|GetActorLocation (Variables|Default|GetAIRef)) (Transformation|GetActorLocation _characterref))) (Math|Vector|GetForwardVector (Variables|/Game/OurStuff/Blueprints/BP_Character.BP_Character_C|GetCamera _characterref))) 0.4 1.0)))

(fn HandlePlayerinRangeSense
  (AI|Components|Blackboard|SetValueasBool (Variables|Default|GetBlackboard) (Utilities|Name|MakeLiteralName "TargetInRange") (Variables|/Game/OurStuff/AI/WeepingAngel/BP_WeepingAngelOrigin.BP_WeepingAngelOrigin_C|GetIsPlayerInRange (Variables|/Game/OurStuff/AI/WeepingAngel/BP_WeepingAngelComponent.BP_WeepingAngelComponent_C|GetOriginArea (Variables|/Game/OurStuff/AI/WeepingAngel/BP_WeepingAngel.BP_WeepingAngel_C|GetBP_WeepingAngelComponent (Variables|Default|GetAIRef))))))